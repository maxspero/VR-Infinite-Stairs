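; BP_Chair is a chair actor that pulls the player pawn toward itself after a trace hit event selects it.
; The hit sets ChairClick, which is never cleared, so Tick moves the pawn whenever it is over 100 units away horizontally.
; Each step scales with distance and delta time, using a (1,1,0) vector rotated by the look-at rotation.
; A node snapping the pawn to the chair's transform is unconnected.
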(event `self.ReceiveBeginPlay`)

(event `self.ReceiveActorBeginOverlap`
  (params (OtherActor :type "Actor Object Reference")))

(event `self.ReceiveTick`
  (params (DeltaSeconds :type "Float (single-precision)"))
  (bind _returnvalue (`GameplayStatics.GetPlayerPawn` 0))
  (bind _returnvalue_2 (`self.K2_GetActorLocation` _returnvalue))
  (bind _returnvalue_3 (`self.GetHorizontalDistanceTo` _returnvalue self))
  (if (`self.ChairClick`)
    (if (< 100.0 _returnvalue_3)
      (`self.K2_SetActorLocation` _returnvalue (+ (`KismetMathLibrary.GreaterGreater_VectorRotator` (* (1.0 1.0 0.0) (* (`GameplayStatics.GetWorldDeltaSeconds`) _returnvalue_3)) (`KismetMathLibrary.FindLookAtRotation` _returnvalue_2 (`SceneComponent.K2_GetComponentLocation` (`self.StaticMeshComponent`)))) _returnvalue_2) false))))

(event `self.Trace Hit Actor With Component`
  (params (Component :type "PrimitiveComponent Object Reference"))
  (set `self.ChairClick` true))

(fn `UserConstructionScript`)